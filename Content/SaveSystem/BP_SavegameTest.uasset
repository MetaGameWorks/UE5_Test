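; Test Blueprint for saving and loading hero rosters with SaveGame objects.
; An SG_Rosters index in the "Rosters" slot lists slot names, each holding an SG_Roster of character classes named by list count.
; BeginPlay loads or creates the index, prints each roster's hero names via blocking class loads and class defaults, then shows UW_Save.
; Functions save, update and fetch rosters, but the sample save calls are disconnected.
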(event EventBeginPlay
  (CallFunction|LoadRosterList)
  (CallFunction|PrintRostersList)
  (CallFunction|ShowLoadWidget))

(event Collision|EventActorBeginOverlap
  (params (OtherActor :type Actor%20Object%20Reference)))

(event EventTick
  (params (DeltaSeconds :type Float%20%28single-precision%29)))

(fn ConstructionScript)

(fn PrintRostersList
  (for (_ _array_index) (Variables|/Game/SaveSystem/SG_Rosters.SG_Rosters_C|GetRostersNames (Variables|Default|GetRosters))
    (Development|PrintString "Hello")
    ;[1 1 1] You can use both
    (bind _characternames (CallFunction|LoadRosterfromIndex _array_index))
    (for (_array_element _array_index_2) _characternames
      (bind _returnvalue (Utilities|LoadClassAssetBlocking _array_element))
      (bind _asbp_hero (Utilities|Casting|CastToBP_HeroClass _returnvalue))
      (Development|PrintString (Utilities|String|Append "  " (Utilities|String|ToString(Integer) _array_index_2) ") " (.HeroName (Utilities|GetClassDefaults _asbp_hero)))))))

(fn SaveNewRoster
  (params (Characters :type Array%20of%20BP%20Hero%20Soft%20Class%20References))
  (bind _rosters (Variables|Default|GetRosters))
  (bind _rosters_2 (Variables|Default|GetRosters))
  (bind _rostersnames (Variables|/Game/SaveSystem/SG_Rosters.SG_Rosters_C|GetRostersNames _rosters_2))
  (bind _returnvalue (Utilities|Array|Length _rostersnames))
  (bind _returnvalue_2 (Utilities|String|ToString(Integer) _returnvalue))
  (bind _returnvalue_3 (Utilities|String|Append "Roster_" _returnvalue_2))
  (bind _returnvalue_4 (SaveGame|CreateSaveGameObject "/Game/SaveSystem/SG_Roster.SG_Roster_C"))
  (Variables|/Game/SaveSystem/SG_Roster.SG_Roster_C|SetCharacters _returnvalue_4 Characters)
  (SaveGame|SaveGametoSlot _returnvalue_4 _returnvalue_3)
  (Utilities|Array|Add (Variables|/Game/SaveSystem/SG_Rosters.SG_Rosters_C|GetRostersNames _rosters) _returnvalue_3)
  (SaveGame|SaveGametoSlot _rosters "Rosters")
  (return))

(fn LoadRosterList
  ;[1 1 1] Load rosters list
  (bind _returnvalue (SaveGame|LoadGamefromSlot "Rosters"))
  (bind _assg_rosters (Utilities|Casting|CastToSG_Rosters _returnvalue)
    (:then
      (Variables|Default|SetRosters _assg_rosters))
    (:CastFailed
      (bind _returnvalue_2 (SaveGame|CreateSaveGameObject "/Game/SaveSystem/SG_Rosters.SG_Rosters_C"))
      (bind _output_get (Variables|Default|SetRosters _returnvalue_2))
      (SaveGame|SaveGametoSlot _output_get "Rosters")))
  (return))

(fn LoadRosterfromName
  (params (SlotName :type String))
  (bind _returnvalue (SaveGame|LoadGamefromSlot SlotName))
  (bind _assg_roster (Utilities|Casting|CastToSG_Roster _returnvalue)
    (:then
      (return (Variables|/Game/SaveSystem/SG_Roster.SG_Roster_C|GetCharacters _assg_roster) true))
    (:CastFailed
      (return 0 false))))

(fn LoadRosterfromIndex
  (params (RosterIndex :type Integer))
  (bind (_characternames _valid) (CallFunction|LoadRosterfromName (Utilities|Array|Get(acopy) (Variables|/Game/SaveSystem/SG_Rosters.SG_Rosters_C|GetRostersNames (Variables|Default|GetRosters)) RosterIndex)))
  (return _characternames _valid))

(fn UpdateRosterbyName
  (params (SlotName :type String) (Roster :type Array%20of%20BP%20Hero%20Soft%20Class%20References))
  (bind _returnvalue (SaveGame|CreateSaveGameObject "/Game/SaveSystem/SG_Roster.SG_Roster_C"))
  (Variables|/Game/SaveSystem/SG_Roster.SG_Roster_C|SetCharacters _returnvalue Roster)
  (bind _returnvalue_2 (SaveGame|SaveGametoSlot _returnvalue SlotName))
  (return _returnvalue_2))

(fn GetRosterList
  (return (Variables|/Game/SaveSystem/SG_Rosters.SG_Rosters_C|GetRostersNames (Variables|Default|GetRosters))))

(fn ShowLoadWidget
  (Utilities|IsValid (Variables|Default|GetSaveWidget)
    (:Is%20Not%20Valid
      (bind _returnvalue (UserInterface|CreateWidget "/Game/SaveSystem/SaveUi/UW_Save.UW_Save_C"))
      (bind _output_get (Variables|Default|SetSaveWidget _returnvalue))
      (UserInterface|Viewport|AddtoViewport _output_get 0))))