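; BP_SaveManager loads or creates the save data for character rosters.
; LoadRosters reads the "Rosters" index save into a variable, or creates and saves a new one and then calls LoadMasterRoster.
; LoadMasterRoster checks for the "_001" roster save and, if absent, fills one from GetDefaultRoster and registers its name in the index.
; The event graph is empty, so nothing here calls LoadRosters itself.
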(event EventBeginPlay)

(event Collision|EventActorBeginOverlap
  (params (OtherActor :type Actor%20Object%20Reference)))

(event EventTick
  (params (DeltaSeconds :type Float%20%28single-precision%29)))

(fn ConstructionScript)

(fn LoadRosters
  (bind _returnvalue (SaveGame|LoadGamefromSlot "Rosters"))
  (bind _assg_rosters (Utilities|Casting|CastToSG_Rosters _returnvalue)
    (:then
      (Variables|Default|SetRosters _assg_rosters))
    (:CastFailed
      (bind _returnvalue_2 (SaveGame|CreateSaveGameObject "/Game/SaveSystem/SG_Rosters.SG_Rosters_C"))
      (bind _output_get (Variables|Default|SetRosters _returnvalue_2))
      (SaveGame|SaveGametoSlot _output_get "Rosters")
      (CallFunction|LoadMasterRoster)))
  (return))

(fn LoadMasterRoster
  (bind _rosters (Variables|Default|GetRosters))
  (bind _returnvalue (SaveGame|LoadGamefromSlot "_001"))
  (Utilities|Casting|CastToSG_Roster _returnvalue
    (:then
      _)
    (:CastFailed
      (bind _returnvalue_2 (SaveGame|CreateSaveGameObject "/Game/SaveSystem/SG_Roster.SG_Roster_C"))
      (Variables|/Game/SaveSystem/SG_Roster.SG_Roster_C|SetCharacters _returnvalue_2 (CallFunction|GetDefaultRoster))
      (SaveGame|SaveGametoSlot _returnvalue_2 "_001")
      (Utilities|Array|Add (Variables|/Game/SaveSystem/SG_Rosters.SG_Rosters_C|GetRostersNames _rosters) "_001")
      (SaveGame|SaveGametoSlot _rosters "Rosters")))
  (return))